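; VR menu pawn that lets motion controllers point at and click world-space widgets, with floor-level tracking origin.
; Left and right press inputs send left-mouse pointer clicks through each hand's WidgetInteraction component.
; On Tick, hovering a MenuWidgetBP widget traces from the right controller and stretches a spline-mesh beam to the hit; otherwise the spline endpoint collapses to its start.
; Matching left-controller beam logic exists but is disconnected and never runs.
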(event `self.ReceiveTick`
  (params (DeltaSeconds :type "Float (single-precision)"))
  (bind _beam2 (`self.Beam2`))
  (bind _widgetinteraction1 (`self.WidgetInteraction1`))
  (bind _motioncontrollerright (`self.MotionControllerRight`))
  (bind _returnvalue (`SceneComponent.K2_GetComponentLocation` _motioncontrollerright))
  (if (`WidgetInteractionComponent.IsOverHitTestVisibleWidget` _widgetinteraction1)
    (cast `/Game/Widgets/MenuWidgetBP` (`ActorComponent.GetOwner` (`WidgetInteractionComponent.GetHoveredWidgetComponent` _widgetinteraction1)))
    (bind (_outhit _returnvalue_2) (`KismetSystemLibrary.LineTraceSingle` _returnvalue (+ _returnvalue (* (`KismetMathLibrary.GetForwardVector` (`SceneComponent.K2_GetComponentRotation` _motioncontrollerright)) (`WidgetInteractionComponent.InteractionDistance` (`self.WidgetInteraction1`)))) "TraceTypeQuery1"))
    (if _returnvalue_2
      (`SplineComponent.SetLocationAtSplinePoint` _beam2 1 (`.Location` (`GameplayStatics.BreakHitResult` _outhit)) "World" true)
      (`SplineMeshComponent.SetStartAndEnd` (`self.SplineMesh1`) (`SplineComponent.GetLocationAtSplinePoint` _beam2 0 "Local") (`SplineComponent.GetTangentAtSplinePoint` _beam2 0 "Local") (`SplineComponent.GetLocationAtSplinePoint` _beam2 1 "Local") (`SplineComponent.GetTangentAtSplinePoint` _beam2 1 "Local") true))
    (else
      (`SplineComponent.SetLocationAtSplinePoint` _beam2 1 (`SplineComponent.GetLocationAtSplinePoint` _beam2 0 "World") "World" true))))

(event `InputAction|MenuP:ressL`
  (params (Key :type "Key Structure"))
  (bind _widgetinteraction (`self.WidgetInteraction`))
  ;[1 1 1] MenuPress Left
  (:`Pressed`
    (`WidgetInteractionComponent.PressPointerKey` _widgetinteraction "LeftMouseButton"))
  (:`Released`
    (`WidgetInteractionComponent.ReleasePointerKey` _widgetinteraction "LeftMouseButton")))

(event `self.ReceiveBeginPlay`
  (`HeadMountedDisplayFunctionLibrary.SetTrackingOrigin` "Floor"))

(event `InputAction|MenuPressR`
  (params (Key :type "Key Structure"))
  (bind _widgetinteraction1 (`self.WidgetInteraction1`))
  ;[1 1 1] MenuPress Right
  (:`Pressed`
    (`WidgetInteractionComponent.PressPointerKey` _widgetinteraction1 "LeftMouseButton"))
  (:`Released`
    (`WidgetInteractionComponent.ReleasePointerKey` _widgetinteraction1 "LeftMouseButton")))

(fn `UserConstructionScript`)